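; ColumnsBP is a building-piece Blueprint that configures a column mesh in the editor according to a floor number choice.
; Its construction script rebuilds the SelectedMesh array from the single column component for each of three enum options, with the second also halving its world Z scale.
; All options then make the column visible, call SetStaticMesh on the MeshIndex entry and print its name.
; The event graph holds no active logic.
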(event EventBeginPlay)

(event Collision|EventActorBeginOverlap
  (params (OtherActor :type Actor%20Object%20Reference)))

(event EventTick
  (params (DeltaSeconds :type Float%20%28single-precision%29)))

(fn ConstructionScript
  (bind _meshindex (Variables|Default|GetMeshIndex))
  (bind _floor_number_choices (Variables|Default|GetFloor%20Number%20Choices))
  (Utilities|FlowControl|Sequence
    (:then_1
      (if (Utilities|Enum|Equal(Enum) _floor_number_choices "NewEnumerator0")
        (Utilities|Array|Clear (Variables|Default|GetSelectedMesh))
        (bind _output_get (Variables|Default|SetSelectedMesh (Utilities|Array|MakeArray (Variables|Default|GetBuildingPieceColumns1))))
        (for _array_element _output_get
          _)
        (if (<= _meshindex (Utilities|Array|Length (Variables|Default|GetSelectedMesh))) :!label _label
          (for _array_element_2 (Variables|Default|GetSelectedMesh)
            (Rendering|SetVisibility _array_element_2 true false))
          (Components|StaticMesh|SetStaticMesh (Utilities|Array|Get(acopy) (Variables|Default|GetSelectedMesh) _meshindex) 0)
          (Rendering|SetVisibility (Utilities|Array|Get(acopy) (Variables|Default|GetSelectedMesh) _meshindex) true false)
          (Development|PrintString (Utilities|GetDisplayName (Utilities|Array|Get(acopy) (Variables|Default|GetSelectedMesh) _meshindex))))
        (elif (Utilities|Enum|Equal(Enum) _floor_number_choices "NewEnumerator1")
          (Utilities|Array|Clear (Variables|Default|GetSelectedMesh))
          (bind _output_get_2 (Variables|Default|SetSelectedMesh (Utilities|Array|MakeArray (Variables|Default|GetBuildingPieceColumns1))))
          (for _array_element_3 _output_get_2
            (Transformation|SetWorldScale3D _array_element_3 "1.000000,1.000000,0.500000"))
          (goto _label)
          (elif (Utilities|Enum|Equal(Enum) _floor_number_choices "NewEnumerator2")
            (Utilities|Array|Clear (Variables|Default|GetSelectedMesh))
            (bind _output_get_3 (Variables|Default|SetSelectedMesh (Utilities|Array|MakeArray (Variables|Default|GetBuildingPieceColumns1))))
            (for _array_element_4 _output_get_3
              _)
            (goto _label)))))))
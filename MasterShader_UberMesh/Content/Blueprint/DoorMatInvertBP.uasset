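; A modular building piece Blueprint whose construction script sets which wall and door meshes show for a chosen floor level.
; It hides the bottom, middle and top component arrays, then selects one by FloorNumberChoices.
; If MeshIndex is at most the array length, it shows that whole array and calls SetStaticMesh with no mesh on the indexed component; otherwise the array stays hidden.
; The event graph holds only disabled placeholder events.
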(event EventBeginPlay)

(event Collision|EventActorBeginOverlap
  (params (OtherActor :type Actor%20Object%20Reference)))

(event EventTick
  (params (DeltaSeconds :type Float%20%28single-precision%29)))

(fn ConstructionScript
  (bind _floor_number_choices (Variables|Default|GetFloor%20Number%20Choices))
  (Utilities|FlowControl|Sequence
    (:then_0
      ;[1 1 1] Bottom Meshes Array
      (bind _output_get (Variables|Default|SetBottomMeshes (Utilities|Array|MakeArray (Variables|Default|GetBuildingPieceSimpleWall01) (Variables|Default|GetBuildingPieceDoor))))
      (for _array_element _output_get
        (Rendering|SetVisibility _array_element false false))
      ;[1 1 1] Middle Meshes Array
      (bind _output_get_2 (Variables|Default|SetMiddleMeshes (Utilities|Array|MakeArray (Variables|Default|GetBuildingPieceMiddleSimpleWall01) (Variables|Default|GetBuildingPieceMiddleWindowWall01))))
      (for _array_element_2 _output_get_2
        (Rendering|SetVisibility _array_element_2 false false))
      ;[1 1 1] Top Meshes Array
      (bind _output_get_3 (Variables|Default|SetTopMeshes (Utilities|Array|MakeArray (Variables|Default|GetBuildingPieceWallTop01))))
      (for _array_element_3 _output_get_3
        (Rendering|SetVisibility _array_element_3 false false))
      ;[1 1 1] Check wich floor is selected and set selectedMesh array
      (if (Utilities|Enum|Equal(Enum) _floor_number_choices "NewEnumerator0")
        (Variables|Default|SetSelectedMesh (Variables|Default|GetBottomMeshes))
        (if (<= (Variables|Default|GetMeshIndex) (Utilities|Array|Length (Variables|Default|GetSelectedMesh))) :!label _label
          (for _array_element_4 (Variables|Default|GetSelectedMesh)
            (Rendering|SetVisibility _array_element_4 true false))
          (Components|StaticMesh|SetStaticMesh (Utilities|Array|Get(acopy) (Variables|Default|GetSelectedMesh) (Variables|Default|GetMeshIndex)) 0)
          (Rendering|SetVisibility (Utilities|Array|Get(acopy) (Variables|Default|GetSelectedMesh) (Variables|Default|GetMeshIndex)) true false)
          (else
            (for _array_element_5 (Variables|Default|GetSelectedMesh)
              (Rendering|SetVisibility _array_element_5 false false))))
        (elif (Utilities|Enum|Equal(Enum) _floor_number_choices "NewEnumerator1")
          (Variables|Default|SetSelectedMesh (Variables|Default|GetMiddleMeshes))
          (goto _label)
          (elif (Utilities|Enum|Equal(Enum) _floor_number_choices "NewEnumerator2")
            (Variables|Default|SetSelectedMesh (Variables|Default|GetTopMeshes))
            (goto _label)))))))